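; BP_AIPath is a spline-based path actor that hands out target points, by its name for AI movement.
; GetNextTargetPoint increments CurrentIndex, wraps it to the first point past the end of the spline, and returns that point's world location.
; The index lives on the path itself, so all callers share one position in the loop.
; The event graph and construction script contain no logic.
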(event EventBeginPlay)

(event Collision|EventActorBeginOverlap
  (params (OtherActor :type Actor%20Object%20Reference)))

(event EventTick
  (params (DeltaSeconds :type Float%20%28single-precision%29)))

(fn ConstructionScript)

(fn GetNextTargetPoint
  (bind _result (Math|Integer|IncrementInt (Variables|Default|GetCurrentIndex))
    (:%20%20
      (if (>= _result (Spline|GetNumberOfSplinePoints (Variables|Default|GetSpline)))
        (Variables|Default|SetCurrentIndex 0))
      (return (Spline|GetLocationatSplinePoint (Variables|Default|GetSpline) (Variables|Default|GetCurrentIndex) "World")))))